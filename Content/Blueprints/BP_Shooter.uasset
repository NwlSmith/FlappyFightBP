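; BP_Shooter is a child Blueprint for an input-driven character or pawn that fires projectiles.
; The LJump input calls CustomMovement, which is not defined in this graph.
; The LShoot input, gated by CanShoot and CanMove, spawns BP_Projectile at the ProjectilePosition transform with a scream sound, then uses a RateOfFire delay as cooldown.
; Overlap and construction logic defer to the parent class.
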(event `InputAction|LJump` :consume false :overrideparent false
  (params (Key :type "Key Structure"))
  (:`Pressed`
    (`self.CustomMovement`)))

(event `InputAction|LShoot`
  (params (Key :type "Key Structure"))
  (:`Pressed`
    (if (and (`self.CanShoot`) (`self.CanMove`))
      (`|SpawnActorFromClass` "/Game/Blueprints/BP_Projectile.BP_Projectile_C" (`SceneComponent.K2_GetComponentToWorld` (`self.ProjectilePosition`)) "Undefined" "OverrideRootScale" null null)
      (`GameplayStatics.PlaySoundAtLocation` "/Game/Audio/comical-screams-01.comical-screams-01" (`SceneComponent.GetSocketLocation` (`self.StaticMesh`) "None") (struct) 1.0 1.0 0.0 null null null)
      (set `self.CanShoot` false)
      (`KismetSystemLibrary.Delay` (`self.RateOfFire`))
      (set `self.CanShoot` true))))

(event `self.ReceiveActorBeginOverlap`
  (params (OtherActor :type "Actor Object Reference"))
  (`parent.ReceiveActorBeginOverlap` OtherActor))

(fn `UserConstructionScript`
  (`parent.UserConstructionScript`))