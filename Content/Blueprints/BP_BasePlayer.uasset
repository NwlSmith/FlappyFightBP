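; Base player for a physics-driven, Flappy Bird-style character with a color-tinted thruster, tilted each tick by vertical velocity.
; CustomMovement, not called here, applies upward force below MaxHeight while movement is allowed, zeroing velocity first unless falling.
; Hitting BP_BoundaryBottom while alive plays explosion and scream, swaps material and freezes the mesh at its start transform.
; After RespawnDelay physics resumes, then a short delay restores the material and alive state.
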(event `self.ReceiveTick`
  (params (DeltaSeconds :type "Float (single-precision)"))
  (if (`SceneComponent.IsSimulatingPhysics` (`self.StaticMesh`) "None")
    (`self.RotateWVel`)))

(event `self.ReceiveHit`
  (params (MyComp :type "PrimitiveComponent Object Reference") (Other :type "Actor Object Reference") (OtherComp :type "PrimitiveComponent Object Reference") (bSelfMoved :type Boolean) (HitLocation :type "Vector Structure") (HitNormal :type "Vector Structure") (NormalImpulse :type "Vector Structure") (Hit :type "HitResult Structure (by ref)"))
  (cast `/Game/Blueprints/BP_BoundaryBottom` Other)
  (if (`self.IsAlive`)
    (bind _returnvalue (`GameplayStatics.SpawnEmitterAtLocation` "/Game/ParticleSystems/PS_SemiCirclularExplosion.PS_SemiCirclularExplosion" (`KismetMathLibrary.TransformLocation` (`SceneComponent.GetSocketTransform` (`self.StaticMesh`) "None" "RTS_World") (10.0 0.0 0.0)) (struct :`Yaw` 90.0)))
    (`FXSystemComponent.SetColorParameter` _returnvalue "PrimaryColor" (`self.PrimaryColor`))
    (`|ExecutionSequence`
      (:`then_0`
        (`self.Reset Movement`))
      (:`then_1`
        (`PrimitiveComponent.SetMaterial` (`self.StaticMesh`) 1 "/Game/Materials/M_DefaultBody.M_DefaultBody") ; Trigger animation instead?
      )
      (:`then_2`
        (`GameplayStatics.PlaySoundAtLocation` "/Game/Audio/comical-screams-01.comical-screams-01" (0.0 0.0 0.0) (struct) 1.0 1.0 0.0 null null null))
      (:`then_3`
        (set `self.IsAlive` false)
        (`KismetSystemLibrary.Delay` (`self.RespawnDelay`))
        (`self.Resume Movement`)
        (`KismetSystemLibrary.Delay` 0.5)
        (`PrimitiveComponent.SetMaterial` (`self.StaticMesh`) 1 (`self.PrimaryColorMat`))
        (set `self.IsAlive` true)))))

(event `self.ReceiveBeginPlay`
  (set `self.StartTransform` (`SceneComponent.GetSocketTransform` (`self.StaticMesh`) "None" "RTS_World"))
  (bind _returnvalue (`GameplayStatics.SpawnEmitterAttached` "/Game/ParticleSystems/PS_Thruster.PS_Thruster" (`self.ThrusterPosition`) "None" (0.0 0.0 0.0) (struct) (1.0 1.0 1.0) "KeepRelativeOffset" false))
  (`FXSystemComponent.SetColorParameter` _returnvalue "PrimaryColor" (`self.PrimaryColor`)))

(fn `AddForceUp`
  (params (Target :type "PrimitiveComponent Object Reference") (`Force Z` :type "Float (double-precision)"))
  (`PrimitiveComponent.AddForce` Target (`KismetMathLibrary.MakeVector` 0.0 0.0 `Force Z`) "None" false))

(fn `CustomMovement`
  (bind (_returnvalue_x _returnvalue_y _returnvalue_z) (`KismetMathLibrary.BreakVector` (`self.GetVelocity`)))
  (bind _staticmesh (`self.StaticMesh`))
  (bind (_returnvalue_x_2 _returnvalue_y_2 _returnvalue_z_2) (`KismetMathLibrary.BreakVector` (`SceneComponent.K2_GetComponentLocation` (`self.StaticMesh`))))
  (if (and (> (`self.MaxHeight`) _returnvalue_z_2) (`self.CanMove`))
    (if (not (< _returnvalue_z 0.0))
      (`PrimitiveComponent.SetPhysicsLinearVelocity` _staticmesh (0.0 0.0 0.0) false "None"))
    (`self.AddForceUp` _staticmesh (`self.JumpPower`))))

(fn `Reset Movement`
  (bind _staticmesh (`self.StaticMesh`))
  (`|ExecutionSequence`
    (:`then_2`
      (set `self.CanMove` false))
    (:`then_3`
      (`SceneComponent.K2_SetWorldTransform` _staticmesh (`self.StartTransform`) false false))
    (:`then_4`
      (`PrimitiveComponent.SetSimulatePhysics` _staticmesh false))
    (:`then_5`
      (`PrimitiveComponent.SetEnableGravity` _staticmesh false))))

(fn `Resume Movement`
  (bind _staticmesh (`self.StaticMesh`))
  (`|ExecutionSequence`
    (:`then_1`
      (`PrimitiveComponent.SetSimulatePhysics` _staticmesh true))
    (:`then_2`
      (set `self.CanMove` true))
    (:`then_3`
      (`PrimitiveComponent.SetEnableGravity` _staticmesh true))))

(fn `RotateWVel`
  (bind _staticmesh (`self.StaticMesh`))
  (bind _returnvalue (`PrimitiveComponent.GetPhysicsLinearVelocity` _staticmesh "None"))
  (`SceneComponent.K2_SetWorldTransform` _staticmesh (`KismetMathLibrary.MakeTransform` (`SceneComponent.GetSocketLocation` _staticmesh "None") (`KismetMathLibrary.MakeRotator` (/ (.z _returnvalue) -40.0))) false false))

(fn `UserConstructionScript`)