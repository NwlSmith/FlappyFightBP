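; BP_Projectile is a shot that destroys mines in a game using the GM_Flappy game mode.
; On spawn it plays an attached firing sound with randomized pitch.
; On overlap it destroys itself at a BP_Boundary; on a BP_Mine it decrements the game mode's Score, refreshes it through UpdateScore and calls the mine's DestroyMe.
; The projectile does not destroy itself when it hits a mine.
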(event `self.ReceiveActorBeginOverlap`
  (params (OtherActor :type "Actor Object Reference"))
  (cast `/Game/Blueprints/BP_Boundary` OtherActor
    (:`then`
      (`self.K2_DestroyActor`))
    (:`CastFailed`
      (bind _asbp_mine (cast `/Game/Blueprints/BP_Mine` OtherActor))
      (bind _asgm_flappy (cast `/Game/Blueprints/GM_Flappy` (`GameplayStatics.GetGameMode`)))
      (bind _result (`/Engine/EditorBlueprintResources/StandardMacros.DecrementInt` (`/Game/Blueprints/GM_Flappy.Score` _asgm_flappy))
        (:`  `
          (set `/Game/Blueprints/GM_Flappy.Score` _result _asgm_flappy)
          (`/Game/Blueprints/GM_Flappy.UpdateScore` _asgm_flappy)
          (`/Game/Blueprints/BP_Mine.DestroyMe` _asbp_mine))))))

(event `self.ReceiveBeginPlay`
  (`GameplayStatics.SpawnSoundAttached` "/Game/Audio/Shoot01.Shoot01" (`self.StaticMesh`) "None" (0.0 0.0 0.0) (struct) "KeepRelativeOffset" false 0.8 (`KismetMathLibrary.RandomFloatInRange` 0.9 1.1) 0.0 null null))

(fn `UserConstructionScript`)