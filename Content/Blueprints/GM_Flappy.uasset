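; Game manager for a Flappy game that tracks a match countdown and which side, left or right, is winning.
; BeginPlay creates the scoreboard widget, hands it a self reference and starts the countdown from GameTime.
; Tick decrements the timer and refreshes its display, with no check for reaching zero.
; UpdateScore turns the sign of a single Score into an L, R or N winner, then refreshes the scoreboard.
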(event `self.ReceiveBeginPlay`
  (bind _returnvalue (`|CreateWidget` "/Game/UI/WBP_Scoreboard1Score.WBP_Scoreboard1Score_C"))
  (`UserWidget.AddToViewport` _returnvalue 0)
  (set `/Game/UI/WBP_Scoreboard1Score.GameManager` self _returnvalue)
  (bind _output_get (set `self.Scoreboard` _returnvalue))
  (`/Game/UI/WBP_Scoreboard1Score.UpdateScore` _output_get)
  (set `self.CountdownTime` (`self.GameTime`))
  (`/Game/UI/WBP_Scoreboard1Score.UpdateTimer` _output_get))

(event `self.ReceiveTick`
  (params (DeltaSeconds :type "Float (single-precision)"))
  (set `self.CountdownTime` (- (`self.CountdownTime`) DeltaSeconds))
  (`/Game/UI/WBP_Scoreboard1Score.UpdateTimer` (`self.Scoreboard`)))

(fn `UpdateScore`
  (bind _score (`self.Score`))
  (if (> _score 0)
    (set `self.WinningPlayer` "L")
    (elif (< _score 0)
      (set `self.WinningPlayer` "R")
      (else
        (set `self.WinningPlayer` "N"))))
  (`/Game/UI/WBP_Scoreboard1Score.UpdateScore` (`self.Scoreboard`)))

(fn `UserConstructionScript`)