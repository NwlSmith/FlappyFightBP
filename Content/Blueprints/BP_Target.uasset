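; BP_Target is a shootable target that reacts to BP_Projectile overlaps and respawns after a delay.
; While alive, a hit spawns a tinted explosion, resets movement, swaps to the default body material and plays a scream.
; It then resumes movement after RespawnDelay, and shortly afterwards restores its colored material and alive state.
; RJump input triggers CustomMovement, and a separate HitByProjectile function sets another material slot to default.
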(event `InputAction|RJump` :consume false :overrideparent false
  (params (Key :type "Key Structure"))
  (:`Pressed`
    (`self.CustomMovement`)))

(event `self.ReceiveActorBeginOverlap`
  (params (OtherActor :type "Actor Object Reference"))
  (cast `/Game/Blueprints/BP_Projectile` OtherActor)
  (if (`self.IsAlive`)
    (bind _returnvalue (`GameplayStatics.SpawnEmitterAtLocation` "/Game/ParticleSystems/PS_CirclularExplosion.PS_CirclularExplosion" (`KismetMathLibrary.TransformLocation` (`SceneComponent.GetSocketTransform` (`self.StaticMesh`) "None" "RTS_World") (-50.0 0.0 0.0)) (struct :`Yaw` 90.0)))
    (`FXSystemComponent.SetColorParameter` _returnvalue "PrimaryColor" (`self.PrimaryColor`))
    (`|ExecutionSequence`
      (:`then_0`
        (`self.Reset Movement`))
      (:`then_1`
        (`PrimitiveComponent.SetMaterial` (`self.StaticMesh`) 1 "/Game/Materials/M_DefaultBody.M_DefaultBody") ; Trigger animation instead?
      )
      (:`then_2`
        (`GameplayStatics.PlaySoundAtLocation` "/Game/Audio/comical-screams-01.comical-screams-01" (0.0 0.0 0.0) (struct) 1.0 1.0 0.0 null null null))
      (:`then_3`
        (set `self.IsAlive` false)
        (`KismetSystemLibrary.Delay` (`self.RespawnDelay`))
        (`self.Resume Movement`)
        (`KismetSystemLibrary.Delay` 0.5)
        (`PrimitiveComponent.SetMaterial` (`self.StaticMesh`) 1 (`self.PrimaryColorMat`))
        (set `self.IsAlive` true)))))

(fn `HitByProjectile`
  (if true
    (`PrimitiveComponent.SetMaterial` (`self.StaticMesh`) 0 "/Game/Materials/M_DefaultBody.M_DefaultBody")))

(fn `UserConstructionScript`
  (`parent.UserConstructionScript`))